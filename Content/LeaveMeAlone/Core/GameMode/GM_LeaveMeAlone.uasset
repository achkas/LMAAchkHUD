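; Game mode for LeaveMeAlone that runs the match countdown and shows the time-up end screen.
; A looping one-second timer decrements GameTime and clears itself at zero.
; If the player still controls an LMADefaultCharacter then, it opens WBP_EndGameTime with UI-only input and a visible cursor.
; A similar delayed death-screen branch using WBP_EndGameDeth is disconnected and never runs.
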(event Custom|CustomEvent
  (bind _returnvalue (Game|GetPlayerController 0))
  (bind _output_get (Variables|Default|SetGame%20Time (- (Variables|Default|GetGame%20Time) 1)))
  (if (== _output_get 0)
    (Utilities|Time|ClearandInvalidateTimerbyHandle (Variables|Default|GetGameTimerHandle))
    (bind _aspc_leave_me_alone (Utilities|Casting|CastToPC_LeaveMeAlone (Game|GetPlayerController 0)))
    (if (Class|GameplayStatics|ObjectIsA (Pawn|GetControlledPawn _aspc_leave_me_alone) "/Script/LeaveMeAlone.LMADefaultCharacter")
      (bind _returnvalue_2 (UserInterface|CreateWidget "/Game/LeaveMeAlone/Widgets/UI/WBP_EndGameTime.WBP_EndGameTime_C"))
      (bind _output_get_2 (Variables|Default|SetEndGame _returnvalue_2))
      (UserInterface|Viewport|AddtoViewport _output_get_2 0)
      (Input|SetInputModeUIOnly _returnvalue _output_get_2 "DoNotLock" false)
      (Variables|/Script/Engine.PlayerController|SetbShowMouseCursor _returnvalue true))))

(event EventBeginPlay
  (bind _returnvalue (Utilities|Time|SetTimerbyEvent (delegate Custom|CustomEvent) 1.0 true))
  (Variables|Default|SetGameTimerHandle _returnvalue))

(event EventTick
  (params (DeltaSeconds :type Float%20%28single-precision%29)))

(fn ConstructionScript)